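; BP_ZoneMedicineProxy relays medicine-use notifications to the Zone Medicine HUD manager.
; It exposes one function per consumable: radioprotector, antidote, PSI protector, Hercules and glucose.
; Each function looks up the BP_ZoneMedicineHUDManager actor with GetActorOfClass on every call and, if valid, forwards to its function of the same name.
; It holds no state or logic of its own, and does nothing when no manager exists.
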(fn ProcessRadioprotectorUsed
  (bind _returnvalue (Actor|GetActorOfClass 0 "/ZoneMedicine/BPScripts/BP_ZoneMedicineHUDManager.BP_ZoneMedicineHUDManager_C"))
  (Utilities|IsValid _returnvalue
    (:Is%20Valid
      (Default|ProcessRadioprotectorUsed _returnvalue))))

(fn ProcessAntidoteUsed
  (bind _returnvalue (Actor|GetActorOfClass 0 "/ZoneMedicine/BPScripts/BP_ZoneMedicineHUDManager.BP_ZoneMedicineHUDManager_C"))
  (Utilities|IsValid _returnvalue
    (:Is%20Valid
      (Default|ProcessAntidoteUsed _returnvalue))))

(fn ProcessPSIProtectorUsed
  (bind _returnvalue (Actor|GetActorOfClass 0 "/ZoneMedicine/BPScripts/BP_ZoneMedicineHUDManager.BP_ZoneMedicineHUDManager_C"))
  (Utilities|IsValid _returnvalue
    (:Is%20Valid
      (Default|ProcessPSIProtectorUsed _returnvalue))))

(fn ProcessHerculesUsed
  (bind _returnvalue (Actor|GetActorOfClass 0 "/ZoneMedicine/BPScripts/BP_ZoneMedicineHUDManager.BP_ZoneMedicineHUDManager_C"))
  (Utilities|IsValid _returnvalue
    (:Is%20Valid
      (Default|ProcessHerculesUsed _returnvalue))))

(fn ProcessGlucoseUsed
  (bind _returnvalue (Actor|GetActorOfClass 0 "/ZoneMedicine/BPScripts/BP_ZoneMedicineHUDManager.BP_ZoneMedicineHUDManager_C"))
  (Utilities|IsValid _returnvalue
    (:Is%20Valid
      (Default|ProcessGlucoseUsed _returnvalue))))